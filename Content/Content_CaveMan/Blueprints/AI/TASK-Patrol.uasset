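; Behavior tree task that sends the owning AI controller to a random location to patrol.
; It takes the combined bounds of the RecastNavMesh actors, randomly widens them on X and Y, and moves toward a random point in that box.
; The task finishes successfully after a fixed short delay, without checking whether the move was valid or completed.
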(event EventReceiveExecuteAI
  (params (OwnerController :type AI%20Controller%20Object%20Reference) (ControlledPawn :type Pawn%20Object%20Reference))
  (bind _returnvalue (Math|Random|RandomFloatinRange 0.0 5e+02))
  (bind _outactors (Actor|GetAllActorsOfClass "/Script/Engine.RecastNavMesh"))
  (bind (_center _boxextent) (Collision|GetActorArrayBounds _outactors))
  (AI|Navigation|MovetoLocation OwnerController (Math|Random|RandomPointinBoundingBox _center (Math|Vector|MakeVector (+ (.X (Math|Vector|BreakVector _boxextent)) _returnvalue) (+ (.Y (Math|Vector|BreakVector _boxextent)) _returnvalue) (.Z (Math|Vector|BreakVector _boxextent)))) -1.0 true true false)
  (Utilities|FlowControl|Delay 2.0)
  (AI|BehaviorTree|FinishExecute true))